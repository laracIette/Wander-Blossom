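; BP_FollowSpline is an air current actor that carries the player along a spline path.
; Overlapping StartCollider with the player's capsule zeroes their velocity and starts a timeline, guarded by HasPlayer against re-entry.
; The timeline sets the player's location by distance along the spline each update, without sweep, with play rate scaled by Speed over spline length.
; On finish it zeroes velocity again and clears the guard.
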(event OnComponentBeginOverlap(StartCollider)
  (params (OverlappedComponent :type Primitive%20Component%20Object%20Reference) (OtherActor :type Actor%20Object%20Reference) (OtherComp :type Primitive%20Component%20Object%20Reference) (OtherBodyIndex :type Integer) (bFromSweep :type Boolean) (SweepResult :type Hit%20Result%20Structure%20%28by%20ref%29))
  (bind _outplayer (Utilities|GetPlayer))
  (bind _spline (Variables|Default|GetSpline))
  (if (== OtherComp (Variables|/Script/Engine.Character|GetCapsuleComponent _outplayer))
    (if (not (Variables|Default|GetbHasPlayer))
      (Variables|Default|SetbHasPlayer true)
      (Variables|/Script/Engine.MovementComponent|SetVelocity (Variables|/Script/Engine.Character|GetCharacterMovement _outplayer) "0, 0, 0")
      (Components|Timeline|SetPlayRate (Variables|Default|GetFollowSplineTimeline) (* (/ 1.0 (Spline|GetSplineLength (Variables|Default|GetSpline))) (* (Variables|Default|GetSpeed) 1e+03)))
      (bind _value (Timeline|FollowSplineTimeline PlayFromStart)
        (:Update
          (Transformation|SetActorLocation _outplayer (Spline|GetLocationatDistanceAlongSpline _spline (* _value (Spline|GetSplineLength _spline)) "World") false false))
        (:Finished
          (Variables|Default|SetbHasPlayer false)
          (Variables|/Script/Engine.MovementComponent|SetVelocity (Variables|/Script/Engine.Character|GetCharacterMovement _outplayer) "0, 0, 0"))))))

(fn ConstructionScript)