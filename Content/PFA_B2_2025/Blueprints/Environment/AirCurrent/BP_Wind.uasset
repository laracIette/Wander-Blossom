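; BP_Wind is an air current volume that pushes the player along a set direction.
; Every tick, while its collider overlaps the player's capsule, it applies a scaled Force to the character movement along the Direction component's forward vector.
; GetForceMultiplier reads the player's BP_Umbrella child actor and makes the push several times stronger when the umbrella is open.
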(event EventTick
  (params (DeltaSeconds :type Float%20%28single-precision%29))
  (bind _outplayer (Utilities|GetPlayer))
  (if (Class|PrimitiveComponent|IsOverlappingComponent (Variables|Default|GetCollider) (Variables|/Script/Engine.Character|GetCapsuleComponent _outplayer))
    (bind _outvalue (CallFunction|GetForceMultiplier))
    (Physics|AddForce (Variables|/Script/Engine.Character|GetCharacterMovement _outplayer) (* _outvalue (Math|Vector|GetForwardVector (Variables|Default|GetDirection)) (* (Variables|Default|GetForce) 5e+04)))))

(fn ConstructionScript)

(fn GetForceMultiplier
  (if (Variables|/Game/PFA_B2_2025/Blueprints/Weapons/Umbrella/BP_Umbrella.BP_Umbrella_C|GetbIsOpened (.AsBP%20Umbrella (Utilities|Casting|CastToBP_Umbrella (Variables|/Script/Engine.ChildActorComponent|GetChildActor (Variables|/Game/PFA_B2_2025/Blueprints/Entities/Player/BP_Player.BP_Player_C|GetUmbrella (Utilities|GetPlayer))))))
    (return 5.0)
    (else
      (return 1.0))))