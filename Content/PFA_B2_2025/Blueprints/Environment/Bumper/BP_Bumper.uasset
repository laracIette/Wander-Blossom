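; BP_Bumper is an environment bumper that launches the player on overlap with their capsule.
; Launch velocity follows the Arrow component's forward vector scaled by Force, overriding Z while adding to XY.
; A timeline animates the mesh scale for the bump feedback.
; Each bump also resets umbrella stamina and dash, and calls AddMaxJumpCount when the player has jumped more than once.
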(event OnComponentBeginOverlap(Collider)
  (params (OverlappedComponent :type Primitive%20Component%20Object%20Reference) (OtherActor :type Actor%20Object%20Reference) (OtherComp :type Primitive%20Component%20Object%20Reference) (OtherBodyIndex :type Integer) (bFromSweep :type Boolean) (SweepResult :type Hit%20Result%20Structure%20%28by%20ref%29))
  (bind _outplayer (Utilities|GetPlayer))
  (if (== OtherComp (Variables|/Script/Engine.Character|GetCapsuleComponent _outplayer))
    (CallFunction|Bump)
    (bind _outvelocity (CallFunction|GetBumpVelocity))
    (Character|LaunchCharacter _outplayer _outvelocity false true)
    (Default|ResetUmbrellaStamina _outplayer)
    (Default|ResetDash _outplayer)
    (if (> (Variables|/Script/Engine.Character|GetJumpCurrentCount _outplayer) 1)
      (Default|AddMaxJumpCount _outplayer 1))))

(event Custom|Bump
  (bind _scale (Timeline|BumpTimeline PlayFromStart)
    (:Update
      (Transformation|SetRelativeScale3D (Variables|Default|GetMeshScale) (Math|Conversions|ToVector(Float) _scale)))))

(fn ConstructionScript)

(fn GetBumpVelocity
  (return (* (Math|Vector|GetForwardVector (Variables|Default|GetArrow)) (* (Variables|Default|GetForce) 1.5e+03))))