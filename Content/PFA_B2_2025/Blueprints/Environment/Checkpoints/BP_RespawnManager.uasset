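; Respawn manager that tracks the current checkpoint and returns the player to it.
; On BeginPlay it binds to checkpoint reached and kill collider overlap events.
; Respawning first reloads the L_Dynamic streaming level with blocking unload and load, then notifies listeners.
; It then delegates to the current checkpoint, or logs an error and calls the player's own Respawn if none is valid.
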(event Custom|UpdateCurrentCheckpoint
  (params (InCheckpoint :type BP%20Checkpoint%20Object%20Reference))
  (Variables|Default|SetCurrentCheckpoint InCheckpoint))

(event Custom|RespawnPlayer
  (Utilities|FlowControl|Sequence
    (:then_0
      (CallFunction|ReloadDynamicLevel))
    (:then_1
      (bind _currentcheckpoint (Variables|Default|GetCurrentCheckpoint)
        (:then
          (Default|RespawnPlayer _currentcheckpoint))
        (:else
          (Development|PrintString "Invalid Checkpoint Index")
          (Default|Respawn (Utilities|GetPlayer)))))))

(event Custom|ReloadDynamicLevel
  (Class|GameplayStatics|UnloadStreamLevelbySoftObjectPtr "/Game/PFA_B2_2025/Levels/Final/L_Dynamic.L_Dynamic" true)
  (Class|GameplayStatics|LoadStreamLevelbySoftObjectPtr "/Game/PFA_B2_2025/Levels/Final/L_Dynamic.L_Dynamic" true true)
  (Default|CallOnReloadDynamicLevel))

(event EventBeginPlay
  (Utilities|FlowControl|Sequence
    (:then_0
      (EventDispatchers|BindEventtoOnReached (Variables|Default|GetCheckpoints) (EventDispatchers|CreateEvent :!event Custom|UpdateCurrentCheckpoint)))
    (:then_1
      (EventDispatchers|BindEventtoOnPlayerOverlap (Variables|Default|GetKillColliders) (EventDispatchers|CreateEvent :!event Custom|RespawnPlayer)))))

(fn ConstructionScript)