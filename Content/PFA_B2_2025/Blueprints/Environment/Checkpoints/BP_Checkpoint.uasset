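; Checkpoint actor that reacts when the player's capsule enters it and can respawn the player at its respawn arrow.
; Every entry fires OnReached and fades in an open-map widget, which fades out on exit via the reversed timeline.
; The first entry also plays an opening montage, then a sound and a temporary timeline-faded "checkpoint reached" widget.
; Mesh animation starts paused until Activate, and NotifySparkle spawns sparkle effects.
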(event OnComponentEndOverlap(Collider)
  (params (OverlappedComponent :type Primitive%20Component%20Object%20Reference) (OtherActor :type Actor%20Object%20Reference) (OtherComp :type Primitive%20Component%20Object%20Reference) (OtherBodyIndex :type Integer))
  (bind _asbp_player (Utilities|Casting|CastToBP_Player OtherActor))
  (if (== (Variables|/Script/Engine.Character|GetCapsuleComponent _asbp_player) OtherComp)
    (CallFunction|HideOpenMapWidget)))

(event OnComponentBeginOverlap(Collider)
  (params (OverlappedComponent :type Primitive%20Component%20Object%20Reference) (OtherActor :type Actor%20Object%20Reference) (OtherComp :type Primitive%20Component%20Object%20Reference) (OtherBodyIndex :type Integer) (bFromSweep :type Boolean) (SweepResult :type Hit%20Result%20Structure%20%28by%20ref%29))
  (bind _asbp_player (Utilities|Casting|CastToBP_Player OtherActor))
  (if (== (Variables|/Script/Engine.Character|GetCapsuleComponent _asbp_player) OtherComp)
    (CallFunction|ShowOpenMapWidget)
    (Default|CallOnReached self)
    (if (not (Variables|Default|GetbIsReached))
      (Variables|Default|SetbIsReached true)
      (Animation|Montage|PlayMontage (Variables|Default|GetMesh) "/Game/PFA_B2_2025/Animations/Checkpoint/AM_CheckpointOpen.AM_CheckpointOpen"
        (:then
          (Audio|PlaySoundatLocation "/Game/PFA_B2_2025/Audio/SFX/Checkpoint/MS_CheckpointReached.MS_CheckpointReached" (Transformation|GetWorldLocation (Variables|Default|GetMesh)) "0, 0, 0" 1.0 1.0 0.0 "/Game/PFA_B2_2025/Audio/SA_DefaultSoundAttenuation.SA_DefaultSoundAttenuation" 0 0 0)
          (CallFunction|ShowCheckpointReachedWidget))))))

(event Custom|Deactivate
  (Variables|/Script/Engine.SkeletalMeshComponent|SetbPauseAnims (Variables|Default|GetMesh) true)
  (Components|Activation|Deactivate (Variables|Default|GetMesh)))

(event Custom|Activate
  (Variables|/Script/Engine.SkeletalMeshComponent|SetbPauseAnims (Variables|Default|GetMesh) false)
  (Components|Activation|Activate (Variables|Default|GetMesh) false))

(event Custom|NotifySparkle
  (bind _spawnsparklesarrow (Variables|Default|GetSpawnSparklesArrow))
  (Niagara|SpawnSystematLocation "/Game/PFA_B2_2025/VFX/Sparkles/NS_Sparkles.NS_Sparkles" (Transformation|GetWorldLocation _spawnsparklesarrow) (Transformation|GetWorldRotation _spawnsparklesarrow)))

(event Custom|RespawnPlayer
  (bind _outplayer (Utilities|GetPlayer))
  (bind _respawnarrow (Variables|Default|GetRespawnArrow))
  (Default|SetRespawnLocationandRotation _outplayer (Transformation|GetWorldLocation _respawnarrow) (Transformation|GetWorldRotation _respawnarrow))
  (Default|Respawn _outplayer))

(event Custom|HideOpenMapWidget
  (bind _opacity (Timeline|ShowOpenMapTimeline Reverse)
    (:Update
      (Widget|SetRenderOpacity (Variables|Default|GetOpenMapWidget) _opacity))))

(event Custom|ShowOpenMapWidget
  (bind _opacity (Timeline|ShowOpenMapTimeline Play)
    (:Update
      (Widget|SetRenderOpacity (Variables|Default|GetOpenMapWidget) _opacity))))

(event Custom|ShowCheckpointReachedWidget
  (bind _returnvalue (UserInterface|CreateWidget "/Game/PFA_B2_2025/Widgets/Map/WBP_CheckpointReached.WBP_CheckpointReached_C"))
  (UserInterface|Viewport|AddtoViewport _returnvalue 0)
  (bind _opacity (Timeline|ShowCheckpointReachedTimeline Play)
    (:Update
      (Widget|SetRenderOpacity _returnvalue _opacity))
    (:Finished
      (Widget|RemovefromParent _returnvalue))))

(event EventBeginPlay
  (CallFunction|Deactivate)
  (bind _returnvalue (UserInterface|CreateWidget "/Game/PFA_B2_2025/Widgets/Map/WBP_OpenMap.WBP_OpenMap_C"))
  (Variables|Default|SetOpenMapWidget _returnvalue)
  (UserInterface|Viewport|AddtoViewport (Variables|Default|GetOpenMapWidget) 0)
  (Widget|SetRenderOpacity (Variables|Default|GetOpenMapWidget) 0.0))

(fn ConstructionScript)