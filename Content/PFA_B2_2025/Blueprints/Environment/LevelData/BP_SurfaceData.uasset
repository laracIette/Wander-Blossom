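; BP_SurfaceData is a level volume that assigns its SurfaceType to the player's CurrentSurfaceType.
; The value is written when the player's capsule begins overlapping Bounds, ignoring other actors and components.
; BeginPlay waits one tick and runs the same overlap check to cover a player who starts inside.
; There is no end-overlap handling, so this volume never resets the type on exit.
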(event OnComponentBeginOverlap(Bounds)
  (params (OverlappedComponent :type Primitive%20Component%20Object%20Reference) (OtherActor :type Actor%20Object%20Reference) (OtherComp :type Primitive%20Component%20Object%20Reference) (OtherBodyIndex :type Integer) (bFromSweep :type Boolean) (SweepResult :type Hit%20Result%20Structure%20%28by%20ref%29))
  (bind _asbp_player (Utilities|Casting|CastToBP_Player OtherActor))
  (if (== (Variables|/Script/Engine.Character|GetCapsuleComponent _asbp_player) OtherComp)
    (Variables|/Game/PFA_B2_2025/Blueprints/Entities/Player/BP_Player.BP_Player_C|SetCurrentSurfaceType _asbp_player (Variables|Default|GetSurfaceType))))

(event EventBeginPlay
  (bind _outplayer (Utilities|GetPlayer))
  (Utilities|FlowControl|DelayUntilNextTick)
  (if (Class|PrimitiveComponent|IsOverlappingComponent (Variables|/Script/Engine.Character|GetCapsuleComponent _outplayer) (Variables|Default|GetBounds))
    (Variables|/Game/PFA_B2_2025/Blueprints/Entities/Player/BP_Player.BP_Player_C|SetCurrentSurfaceType _outplayer (Variables|Default|GetSurfaceType))))

(fn ConstructionScript)