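; BP_Angler is a moving environment actor that tilts in pitch when activated and tilts back when deactivated.
; At BeginPlay it sets the timeline play rate from Speed, stores its starting rotation and binds to a valid Activable's activate and deactivate events.
; A timeline plays forward or in reverse, adding an Alpha-scaled Angle to the starting pitch, with IsActivated blocking repeat triggers.
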(event Custom|Activate
  (if (not (Variables|Default|GetbIsActivated))
    (Variables|Default|SetbIsActivated true)
    (bind _alpha (Timeline|AngleTimeline Play)
      (:Update
        (Transformation|SetActorRotation (Math|Rotator|MakeRotator (.roll (stale EventBeginPlay _returnvalue)) (+ (.pitch (stale EventBeginPlay _returnvalue)) (* _alpha (Variables|Default|GetAngle))) (.yaw (stale EventBeginPlay _returnvalue))))))))

(event Custom|Deactivate
  (if (Variables|Default|GetbIsActivated)
    (Variables|Default|SetbIsActivated false)
    (bind _alpha (Timeline|AngleTimeline Reverse)
      (:Update
        (Transformation|SetActorRotation (Math|Rotator|MakeRotator (.roll (stale EventBeginPlay _returnvalue)) (+ (.pitch (stale EventBeginPlay _returnvalue)) (* _alpha (Variables|Default|GetAngle))) (.yaw (stale EventBeginPlay _returnvalue))))))))

(event EventBeginPlay
  (Components|Timeline|SetPlayRate (Variables|Default|GetAngleTimeline) (/ 1.0 (Variables|Default|GetSpeed)))
  (bind _returnvalue (Transformation|GetActorRotation))
  (bind _activable (Variables|Default|GetActivable)
    (:then
      (EventDispatchers|BindEventtoOnActivate _activable (EventDispatchers|CreateEvent :!event Custom|Activate))
      (EventDispatchers|BindEventtoOnDeactivate _activable (EventDispatchers|CreateEvent :!event Custom|Deactivate)))
    (:else)))

(fn ConstructionScript)