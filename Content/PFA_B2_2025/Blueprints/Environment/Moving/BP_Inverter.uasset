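; BP_Inverter is a moving environment actor that periodically flips itself, and the actors attached to it, around the roll axis.
; A looping, offset timer drives Invert, which plays a shake timeline along relative X as a warning, then a timeline that adds an angle to the starting roll.
; Attached actors lose collision during the rotation and regain it afterwards.
; Timeline play rates are derived from the speed and duration variables.
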(event Custom|Invert
  (bind _x (Timeline|ShakeTimeline PlayFromStart)
    (:Update
      (Transformation|SetActorRelativeLocation (+ (Variables|Default|GetStartLocation) (Math|Vector|MakeVector (* _x (Variables|Shake|GetShakeRange) 6.0) 0.0 0.0))))
    (:Finished
      (Utilities|FlowControl|Sequence
        (:then_0
          ;[0.15 0.15 0.15 0.5] Disable Collisions
          (for _array_element (Actor|GetAttachedActors true true)
            (Collision|SetActorEnableCollision _array_element false)))
        (:then_1
          (bind _returnvalue (Transformation|GetActorRotation))
          (bind _angle (Timeline|InvertTimeline PlayFromStart)
            (:Update
              (Transformation|SetActorRotation (Math|Rotator|MakeRotator (+ _angle (.roll _returnvalue)) 0.0 0.0)))
            (:Finished
              ;[0.15 0.15 0.15 0.5] Enable Collisions
              (for _array_element_2 (Actor|GetAttachedActors true true)
                (Collision|SetActorEnableCollision _array_element_2 true)))))))))

(event EventBeginPlay
  (Utilities|Time|SetTimerbyEvent (EventDispatchers|CreateEvent :!event Custom|Invert) (+ (Variables|Invert|GetInvertFrequency) (Variables|Invert|GetInvertSpeed)) true false (Variables|Default|GetOffset))
  (Components|Timeline|SetPlayRate (Variables|Default|GetInvertTimeline) (/ 1.0 (Variables|Invert|GetInvertSpeed)))
  (Components|Timeline|SetPlayRate (Variables|Default|GetShakeTimeline) (/ 1.0 (Variables|Shake|GetShakeDuration)))
  (Variables|Default|SetStartLocation (Variables|/Script/Engine.SceneComponent|GetRelativeLocation (Variables|Default|GetDefaultRoot))))

(fn ConstructionScript)