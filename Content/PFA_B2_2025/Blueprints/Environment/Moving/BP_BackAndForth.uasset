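; Environment actor that moves along its direction arrow, scaled by Range, as a back-and-forth mover switched on and off by activation events.
; BeginPlay caches the root's relative start location, sets the timeline play rate to the inverse of Frequency and binds to a valid Activable's activate/deactivate events.
; Activate plays the timeline, whose Alpha offsets the actor from its start without sweeping.
; Deactivate stops the timeline in place.
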(event Custom|Activate
  (bind _alpha (Timeline|AnimationTimeline Play)
    (:Update
      (Transformation|SetActorRelativeLocation (+ (Variables|Default|GetStartLocation) (* _alpha (Math|Vector|GetForwardVector (Variables|Default|GetDirectionArrow)) (Variables|Default|GetRange)))))))

(event Custom|Deactivate
  (bind _alpha (Timeline|AnimationTimeline Stop)
    (:Update
      (Transformation|SetActorRelativeLocation (+ (Variables|Default|GetStartLocation) (* _alpha (Math|Vector|GetForwardVector (Variables|Default|GetDirectionArrow)) (Variables|Default|GetRange)))))))

(event EventBeginPlay
  (Utilities|FlowControl|Sequence
    (:then_0
      (Variables|Default|SetStartLocation (Variables|/Script/Engine.SceneComponent|GetRelativeLocation (Variables|Default|GetDefaultSceneRoot)))
      (Components|Timeline|SetPlayRate (Variables|Default|GetAnimationTimeline) (/ 1.0 (Variables|Default|GetFrequency))))
    (:then_1
      (bind _activable (Variables|Default|GetActivable)
        (:then
          (EventDispatchers|BindEventtoOnActivate _activable (EventDispatchers|CreateEvent :!event Custom|Activate))
          (EventDispatchers|BindEventtoOnDeactivate _activable (EventDispatchers|CreateEvent :!event Custom|Deactivate)))
        (:else)))))

(fn ConstructionScript)