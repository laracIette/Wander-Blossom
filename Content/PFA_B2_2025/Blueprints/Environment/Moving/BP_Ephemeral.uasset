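; BP_Ephemeral is an environment platform that breaks after the player steps on it, then respawns.
; A player capsule overlap on DestroyCollider starts a delay, then plays a breaking-rocks montage, with a flag blocking retriggers.
; The NotifyBreak event disables StepCollider collision and signals destruction.
; When the montage completes, the mesh hides, then after a respawn delay returns with collision and signals respawn.
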(event OnComponentBeginOverlap(DestroyCollider)
  (params (OverlappedComponent :type Primitive%20Component%20Object%20Reference) (OtherActor :type Actor%20Object%20Reference) (OtherComp :type Primitive%20Component%20Object%20Reference) (OtherBodyIndex :type Integer) (bFromSweep :type Boolean) (SweepResult :type Hit%20Result%20Structure%20%28by%20ref%29))
  (if (not (Variables|Default|GetbIsDestroyed))
    (bind _asbp_player (Utilities|Casting|CastToBP_Player OtherActor))
    (if (== (Variables|/Script/Engine.Character|GetCapsuleComponent _asbp_player) OtherComp)
      (Variables|Default|SetbIsDestroyed true)
      (Utilities|FlowControl|Delay (Variables|Default|GetDelayBeforeDesctruction))
      (Animation|Montage|PlayMontage (Variables|Default|GetMesh) "/Game/PFA_B2_2025/Animations/BreakingRocks/AM_BreakingRocksBreak.AM_BreakingRocksBreak"
        (:OnCompleted
          (Rendering|SetVisibility (Variables|Default|GetMesh) false false)
          ;[0.15 0.15 0.15 0.5] Respawn
          (Utilities|FlowControl|Delay (Variables|Default|GetDelayBeforeRespawn))
          (Variables|Default|SetbIsDestroyed false)
          (Collision|SetCollisionEnabled (Variables|Default|GetStepCollider) "QueryAndPhysics")
          (Rendering|SetVisibility (Variables|Default|GetMesh) true false)
          (Default|CallOnRespawn))))))

(event Custom|NotifyBreak
  ;[0.15 0.15 0.15 0.5] Destroy
  (Collision|SetCollisionEnabled (Variables|Default|GetStepCollider) "NoCollision")
  (Default|CallOnDestroy))

(fn ConstructionScript)

(fn Show)