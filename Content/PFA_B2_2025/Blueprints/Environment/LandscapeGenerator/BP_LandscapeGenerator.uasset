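; Landscape generator actor that scatters non-colliding instanced static meshes between an inner and outer box when its construction script runs.
; Separate seeded random streams drive weighted mesh choice, location, rotation within an up-facing cone, and scale.
; Points inside the inner box are re-rolled, and each mesh type gets one cached instanced component.
; Scale combines random range, Perlin noise and a factor that grows with horizontal distance from the origin.
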(fn ConstructionScript
  ;[0.15 0.15 0.15 0.5] Random Streams
  (Math|Random|SetRandomStreamSeed (Variables|Default|GetRandomLocationStream) (Variables|Default|GetRandomLocationSeed))
  (Math|Random|SetRandomStreamSeed (Variables|Default|GetRandomMeshStream) (Variables|Default|GetRandomMeshSeed))
  (Math|Random|SetRandomStreamSeed (Variables|Default|GetRandomRotationStream) (Variables|Default|GetRandomRotationSeed))
  (Math|Random|SetRandomStreamSeed (Variables|Default|GetRandomScaleStream) (Variables|Default|GetRandomScaleSeed))
  (CallFunction|AddBoxCollisionComponent (Variables|Default|GetInnerBounds))
  (CallFunction|AddBoxCollisionComponent (Variables|Default|GetOuterBounds))
  (for _index (range 1 (Variables|Default|GetCount))
    (CallFunction|GenerateMeshInstance (CallFunction|GetRandomMesh))))

(fn GenerateMeshInstance
  (params (InMesh :type Static%20Mesh%20Object%20Reference))
  (bind _scalerange (Variables|Default|GetScaleRange))
  (bind _value (CallFunction|GetInstancedStaticMeshComponent InMesh))
  (bind _outlocation (CallFunction|GetRandomLocationinBounds))
  (Components|InstancedStaticMesh|AddInstance _value (Math|Transform|MakeTransform _outlocation (Math|Rotator|MakeRotfromZ (Math|Random|RandomUnitVectorinConeinDegreesfromStream (Variables|Default|GetRandomRotationStream) (Math|Vector|VectorUp) (Variables|Default|GetMaxAngle))) (Math|Conversions|ToVector(Float) (* (CallFunction|GetNoiseValueatLocation _outlocation) (Math|Random|RandomFloatinRangefromStream (Variables|Default|GetRandomScaleStream) (.value (.lowerbound _scalerange)) (.value (.upperbound _scalerange))) (Math|Float|Max(Float) (Math|Float|Power (/ (Math|Vector|VectorLengthXY _outlocation) 2e+05) (Variables|Default|GetScaleOverDistanceFactor)) 1.0) (Variables|Default|GetScaleMultiplier)))) false))

(fn GetRandomLocationinBounds
  (bind _returnvalue (Class|KismetMathLibrary|RandomPointinBoundingBoxfromStream (Variables|Default|GetRandomLocationStream) "0, 0, 0" (Variables|Default|GetOuterBounds) :!label _label))
  (if (CallFunction|GetIsinBounds _returnvalue (Variables|Default|GetInnerBounds))
    (goto _label)
    (else
      (return _returnvalue))))

(fn GetRandomMesh
  (Utilities|FlowControl|Sequence
    (:then_0
      (bind _values (Utilities|Map|Values (Variables|Default|GetMeshes)))
      (for _array_element _values
        (LocalVariables|SetTotalWeight (+ _array_element (LocalVariables|GetTotalWeight)))))
    (:then_1
      (bind _returnvalue (Math|Random|RandomFloatinRangefromStream (Variables|Default|GetRandomMeshStream) 0.0 (LocalVariables|GetTotalWeight)))
      (bind _values_2 (Utilities|Map|Values (Variables|Default|GetMeshes)))
      (for (_array_element_2 _array_index) _values_2
        (bind _output_get (LocalVariables|SetAccumulator (+ _array_element_2 (LocalVariables|GetAccumulator))))
        (if (> _output_get _returnvalue)
          (bind _keys (Utilities|Map|Keys (Variables|Default|GetMeshes)))
          (return (Utilities|Array|Get(acopy) _keys _array_index)))))))

(fn GetInstancedStaticMeshComponent
  (params (InStaticMesh :type Static%20Mesh%20Object%20Reference%20%28by%20ref%29))
  (bind _staticmeshinstancedcomponents (Variables|Default|GetStaticMeshInstancedComponents))
  (bind (_value _returnvalue) (Utilities|Map|Find _staticmeshinstancedcomponents InStaticMesh))
  (if _returnvalue
    (return _value)
    (else
      (bind _returnvalue_2 (AddComponent|AddInstancedStaticMeshComponent false))
      (Collision|SetCollisionEnabled _returnvalue_2 "NoCollision")
      (Components|StaticMesh|SetStaticMesh _returnvalue_2 InStaticMesh)
      (Transformation|SetMobility _returnvalue_2 "Static")
      (Utilities|Map|Add (Variables|Default|GetStaticMeshInstancedComponents) InStaticMesh _returnvalue_2)
      (return _returnvalue_2))))

(fn GetIsinBounds
  (params (InLocation :type Vector) (InBounds :type Vector))
  (return (Class|KismetMathLibrary|BoxIsPointInside (Class|KismetMathLibrary|MakeBoxwithOrigin (Math|Vector|VectorZero) InBounds) InLocation)))

(fn AddBoxCollisionComponent
  (params (InExtent :type Vector))
  (bind _returnvalue (AddComponent|AddBoxComponent false))
  (Components|Box|SetBoxExtent _returnvalue InExtent false)
  (Collision|SetCollisionEnabled _returnvalue "NoCollision"))

(fn GetNoiseValueatLocation
  (params (InLocation :type Vector))
  (bind _noisescale (Variables|Default|GetNoiseScale))
  (bind _noisemultiplierrange (Variables|Default|GetNoiseMultiplierRange))
  (bind _returnvalue (/ InLocation _noisescale))
  (return (Math|Vector|VectorLength (Class|KismetAnimationLibrary|MakePerlinNoiseVectorandRemap (.x _returnvalue) (.y _returnvalue) (.z _returnvalue) (.value (.lowerbound _noisemultiplierrange)) (.value (.upperbound _noisemultiplierrange)) (.value (.lowerbound _noisemultiplierrange)) (.value (.upperbound _noisemultiplierrange)) (.value (.lowerbound _noisemultiplierrange)) (.value (.upperbound _noisemultiplierrange))))))