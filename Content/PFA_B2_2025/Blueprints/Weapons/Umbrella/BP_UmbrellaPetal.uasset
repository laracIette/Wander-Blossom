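; BP_UmbrellaPetal is a single petal actor of the umbrella weapon, holding its Open and IsReady state and playing its animation montages.
; It becomes ready three seconds after BeginPlay, or as soon as the inflate montage starts, which also sets it fully open.
; The fall montage detaches the petal in world space at start and destroys it on completion.
; Inflation can be stopped with a short blend-out.
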(event Custom|StopInflateAnim
  (Animation|Montage|MontageStop (Components|SkeletalMesh|GetAnimInstance (Variables|Default|GetSkeletalMesh)) 0.25 "/Game/PFA_B2_2025/Animations/Umbrella2/Petal/AM_UmbrellaPetalInflate.AM_UmbrellaPetalInflate"))

(event Custom|PlayFallAnim
  (Animation|Montage|PlayMontage (Variables|Default|GetSkeletalMesh) "/Game/PFA_B2_2025/Animations/Umbrella2/Petal/AM_UmbrellaPetalFall.AM_UmbrellaPetalFall"
    (:then
      (Transformation|DetachFromActor "KeepWorld" "KeepWorld" "KeepWorld"))
    (:OnCompleted
      (Actor|DestroyActor))))

(event Custom|PlayInflateAnim
  (Animation|Montage|PlayMontage (Variables|Default|GetSkeletalMesh) "/Game/PFA_B2_2025/Animations/Umbrella2/Petal/AM_UmbrellaPetalInflate.AM_UmbrellaPetalInflate" 1.0 0.0 "Start"
    (:then
      (Variables|Default|SetbIsReady true)
      (Variables|Default|SetOpen 1.0))))

(event Custom|SetOpen
  (params (InValue :type Float%20%28double-precision%29))
  (Variables|Default|SetOpen InValue))

(event EventBeginPlay
  (Utilities|FlowControl|Delay 3.0)
  (Variables|Default|SetbIsReady true))

(fn ConstructionScript)