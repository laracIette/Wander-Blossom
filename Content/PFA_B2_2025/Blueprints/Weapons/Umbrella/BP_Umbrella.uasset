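; BP_Umbrella is an umbrella weapon that opens and closes, deflects projectiles and throws petals.
; Open and Close swap collision between two colliders and drive a morph-target timeline, and hits on the open collider push BP_Projectile meshes with an amplified impulse.
; Petals form a round-robin pool with per-petal cooldown timestamps.
; Throws spawn a BP_Petal toward an actor or direction when the current slot is ready, while DropPetals consumes slots without spawning.
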(event OnComponentHit(OpenedCollider)
  (params (HitComponent :type Primitive%20Component%20Object%20Reference) (OtherActor :type Actor%20Object%20Reference) (OtherComp :type Primitive%20Component%20Object%20Reference) (NormalImpulse :type Vector :default "0, 0, 0") (Hit :type Hit%20Result%20Structure%20%28by%20ref%29))
  (bind _asbp_projectile (Utilities|Casting|CastToBP_Projectile OtherActor))
  (Physics|AddImpulse (Variables|/Game/PFA_B2_2025/Blueprints/Projectiles/BP_Projectile.BP_Projectile_C|GetMesh _asbp_projectile) (* NormalImpulse (Math|Float|MakeLiteralFloat 5.0)) "None" false))

(event Custom|Open
  (if (not (Variables|Default|GetbIsOpened))
    (Collision|SetCollisionEnabled (Variables|Default|GetOpenedCollider) "QueryAndPhysics")
    (Collision|SetCollisionEnabled (Variables|Default|GetClosedCollider) "NoCollision")
    (Variables|Default|SetbIsOpened true)
    (bind _value (Timeline|OpenUmbrellaTimeline Play)
      (:Update
        (Components|SkeletalMesh|SetMorphTarget (Variables|Default|GetUmbrellaMesh) "Open" _value true)))))

(event Custom|Close
  (if (Variables|Default|GetbIsOpened)
    (Collision|SetCollisionEnabled (Variables|Default|GetOpenedCollider) "NoCollision")
    (Collision|SetCollisionEnabled (Variables|Default|GetClosedCollider) "QueryAndPhysics")
    (Variables|Default|SetbIsOpened false)
    (bind _value (Timeline|OpenUmbrellaTimeline Reverse)
      (:Update
        (Components|SkeletalMesh|SetMorphTarget (Variables|Default|GetUmbrellaMesh) "Open" _value true)))))

(event Custom|ThrowPetalAtActor
  (params (InActor :type Actor%20Object%20Reference))
  (bind (_boutresult _returnvalue) (CallFunction|TrySpawnPetal))
  (if _boutresult
    (Default|MovetoActor _returnvalue InActor)))

(event Custom|ThrowPetalAtDirection
  (params (InDirection :type Vector))
  (bind (_boutresult _returnvalue) (CallFunction|TrySpawnPetal))
  (if _boutresult
    (Default|MoveAlongDirection _returnvalue InDirection)))

(event Custom|DropPetals
  (params (InAmount :type Integer))
  (for _index (range 1 InAmount)
    (CallFunction|UseCurrentPetal)))

(event EventBeginPlay
  ;[0.15 0.15 0.15 0.5] Explicitely Close
  (Variables|Default|SetbIsOpened true)
  (CallFunction|Close)
  ;[0.15 0.15 0.15 0.5] Init Petal Times
  (for _index (range 1 (Variables|Default|GetPetals))
    (Utilities|Array|Add (Variables|Default|GetPetalReloadTimes) -9999.0)))

(fn ConstructionScript)

(fn GetCanThrow
  (return (> (- (Utilities|Time|GetGameTimeinSeconds) (Utilities|Array|Get(acopy) (Variables|Default|GetPetalReloadTimes) (Variables|Default|GetCurrentPetal))) (Variables|Default|GetPetalReloadTime))))

(fn UseCurrentPetal
  (Utilities|Array|SetArrayElem (Variables|Default|GetPetalReloadTimes) (Variables|Default|GetCurrentPetal) (Utilities|Time|GetGameTimeinSeconds))
  (Development|PrintText (Utilities|Text|FormatText "Used Petal {Petal}" (Variables|Default|GetCurrentPetal)))
  (CallFunction|SetCurrentPetal (+ (Variables|Default|GetCurrentPetal) 1)))

(fn SetCurrentPetal
  (params (InValue :type Integer))
  (Variables|Default|SetCurrentPetal (Math|Integer|%(Integer) InValue (Variables|Default|GetPetals))))

(fn TrySpawnPetal
  (if (CallFunction|GetCanThrow)
    (CallFunction|UseCurrentPetal)
    (bind _returnvalue (Game|SpawnActorfromClass "/Game/PFA_B2_2025/Blueprints/Weapons/Umbrella/BP_Petal.BP_Petal_C" (Transformation|GetWorldTransform (Variables|Default|GetPetalSpawn)) "Undefined" "MultiplyWithRoot" 0 0))
    (return true _returnvalue)
    (else
      (return false 0))))