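; BP_Petal is a projectile of the Umbrella weapon that damages enemies and triggers world objects.
; It either homes on an actor via a distance-scaled timeline with a randomly tilted arc, or flies straight on Tick.
; Overlaps knock back guards through their attack collider, damage other enemies, activate BP_Activable actors and destroy permitted destructibles.
; Hits destroy the petal, usually with a Niagara burst, adding a break sound on static meshes and protected destructibles.
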(event OnComponentBeginOverlap(DamageCollider)
  (params (OverlappedComponent :type Primitive%20Component%20Object%20Reference) (OtherActor :type Actor%20Object%20Reference) (OtherComp :type Primitive%20Component%20Object%20Reference) (OtherBodyIndex :type Integer) (bFromSweep :type Boolean) (SweepResult :type Hit%20Result%20Structure%20%28by%20ref%29))
  (bind _asbp_guard_enemy (Utilities|Casting|CastToBP_GuardEnemy OtherActor)
    (:then
      (if (== (Variables|/Game/PFA_B2_2025/Blueprints/Entities/Enemies/BP_GuardEnemy.BP_GuardEnemy_C|GetAttackCollider _asbp_guard_enemy) OtherComp)
        (Character|LaunchCharacter _asbp_guard_enemy (* (Math|Vector|Normalize (Math|Vector|MakeVector (.x (Math|Vector|GetUnitDirection(Vector) (Transformation|GetActorLocation) (Transformation|GetActorLocation _asbp_guard_enemy))) (.y (Math|Vector|GetUnitDirection(Vector) (Transformation|GetActorLocation) (Transformation|GetActorLocation _asbp_guard_enemy))) 0.1)) (Variables|Default|GetLaunchGuardForce)) true false)
        (Default|Knockback _asbp_guard_enemy)
        (Actor|DestroyActor :!label _label)))
    (:CastFailed
      (bind _asbp_enemy (Utilities|Casting|CastToBP_Enemy OtherActor)
        (:then
          (if (== OtherComp (Variables|/Script/Engine.Character|GetCapsuleComponent _asbp_enemy))
            (bind _outdamagereceived (Default|ReceiveDamage (Variables|/Game/PFA_B2_2025/Blueprints/Entities/Enemies/BP_Enemy.BP_Enemy_C|GetHealthComponent _asbp_enemy) 1))
            (if (> _outdamagereceived 0)
              (Niagara|SpawnSystematLocation (Variables|Default|GetPetalBurstNiagaraSystem) (Transformation|GetActorLocation) :!label _label_2)
              (goto _label))))
        (:CastFailed
          (bind _asbp_activable (Utilities|Casting|CastToBP_Activable OtherActor)
            (:then
              (Default|Interact _asbp_activable)
              (goto _label_2))
            (:CastFailed
              (bind _asbp_destructible (Utilities|Casting|CastToBP_Destructible OtherActor)
                (:then
                  (if (Variables|/Game/PFA_B2_2025/Blueprints/Interactables/Destructibles/BP_Destructible.BP_Destructible_C|GetbCanBeDestroyedByPlayer _asbp_destructible)
                    (Default|Destroy _asbp_destructible)
                    (goto _label_2)
                    (else
                      _)))
                (:CastFailed
                  (Utilities|Casting|CastToStaticMeshActor OtherActor)))
              (Default|Play3D (Variables|Default|GetBreakSoundComponent))
              (goto _label_2))))))))

(event Custom|MoveAlongDirection
  (params (InDirection :type Vector))
  (Variables|Default|SetThrowDirection (Math|Vector|Normalize InDirection))
  (Variables|Default|SetbIsMovingAlongDirection true))

(event Custom|MoveToActor
  (params (InActor :type Actor%20Object%20Reference))
  (Components|Timeline|SetPlayRate (Variables|Default|GetMoveToLocationTimeline) (* (/ (Components|Timeline|GetTimelineLength (Variables|Default|GetMoveToLocationTimeline)) (Transformation|GetDistanceTo InActor)) (Variables|Default|GetThrowSpeed)))
  (bind _outangle (CallFunction|GetThrowAngle (Transformation|GetActorLocation InActor)))
  (bind _returnvalue (Transformation|GetActorLocation))
  (bind (_direction _alpha _arcvalue) (Timeline|MoveToLocationTimeline Play)
    (:Update
      (Transformation|SetActorLocation (+ (Math|Vector|Lerp(Vector) _returnvalue (Transformation|GetActorLocation InActor) _alpha) (* _arcvalue _outangle (Variables|Default|GetArcHeight))) false false))))

(event EventTick
  (params (DeltaSeconds :type Float%20%28single-precision%29))
  (if (Variables|Default|GetbIsMovingAlongDirection)
    (Transformation|AddActorWorldOffset (* (Variables|Default|GetThrowDirection) (Variables|Default|GetThrowSpeed) (Utilities|Time|GetWorldDeltaSeconds)))))

(fn ConstructionScript)

(fn GetTimeSinceThrow
  (return (- (Utilities|Time|GetGameTimeinSeconds) (Variables|Default|GetLastThrowTime))))

(fn GetThrowAngle
  (params (InTargetLocation :type Vector))
  (return (Math|Vector|Normalize (Math|Vector|RotateVector (Math|Vector|MakeVector 0.0 (Math|Random|RandomFloatinRange -1.0 1.0) 1.0) (Math|Rotator|MakeRotfromX (Math|Vector|GetUnitDirection(Vector) (Transformation|GetActorLocation) InTargetLocation))))))