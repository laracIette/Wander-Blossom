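; AC_SoundComponent is an actor component that plays a configured sound, either non-spatialized or in the world.
; It supplies its Sound, VolumeMultiplier and PitchMultiplier variables to both playback functions.
; Play2D plays the sound in 2D with a caller-provided UI sound flag, while Play3D plays it once at the owner's current location and rotation.
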(fn Play2D
  (params (bIsUISound :type Boolean))
  (Audio|PlaySound2D (Variables|Default|GetSound) (Variables|Default|GetVolumeMultiplier) (Variables|Default|GetPitchMultiplier) 0.0 0 0 bIsUISound))

(fn Play3D
  (bind _returnvalue (Components|GetOwner))
  (Audio|PlaySoundatLocation (Variables|Default|GetSound) (Transformation|GetActorLocation _returnvalue) (Transformation|GetActorRotation _returnvalue) (Variables|Default|GetVolumeMultiplier) (Variables|Default|GetPitchMultiplier) 0.0 0 0 0 0))