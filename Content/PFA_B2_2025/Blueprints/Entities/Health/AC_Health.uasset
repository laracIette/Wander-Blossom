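; Health component for entities, tracking an integer health value between a minimum and maximum and starting at max on BeginPlay.
; SetHealth clamps the value and fires health-changed and death events; AddHealth and RemoveHealth route through it.
; ReceiveDamage applies damage only while alive and damageable, broadcasting and returning the amount actually lost.
; SetToMaxHealth and SetToMinHealth write the value directly, so they fire no events.
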(event EventBeginPlay
  (Variables|Default|SetCurrentHealth (Variables|Default|GetMaxHealth)))

(fn GetIsAlive
  (return (> (Variables|Default|GetCurrentHealth) (Variables|Default|GetMinHealth))))

(fn ReceiveDamage
  (params (InAmount :type Integer))
  (bind _previoushealth (Variables|Default|GetPreviousHealth))
  (bind _currenthealth (Variables|Default|GetCurrentHealth))
  (bind _returnvalue (- _previoushealth _currenthealth))
  (if (CallFunction|GetIsAlive)
    (if (Variables|Default|GetbCanReceiveDamage)
      (CallFunction|SetHealth (- (Variables|Default|GetCurrentHealth) InAmount))
      (if (> _returnvalue 0)
        (Default|CallOnReceiveDamage _returnvalue))
      (return _returnvalue)
      (else
        (return 0)))
    (else
      (return 0))))

(fn SettoMaxHealth
  (Variables|Default|SetCurrentHealth (Variables|Default|GetMaxHealth)))

(fn SettoMinHealth
  (Variables|Default|SetCurrentHealth (Variables|Default|GetMinHealth)))

(fn SetHealth
  (params (InAmount :type Integer))
  (Variables|Default|SetPreviousHealth (Variables|Default|GetCurrentHealth))
  (bind _output_get (Variables|Default|SetCurrentHealth (Math|Integer|Clamp(Integer) InAmount (Variables|Default|GetMinHealth) (Variables|Default|GetMaxHealth))))
  (if (!= _output_get (Variables|Default|GetPreviousHealth))
    (Default|CallOnHealthChanged)
    (if (not (CallFunction|GetIsAlive))
      (Default|CallOnDie))))

(fn AddHealth
  (params (InAmount :type Integer))
  (CallFunction|SetHealth (+ InAmount (Variables|Default|GetCurrentHealth))))

(fn RemoveHealth
  (params (InAmount :type Integer))
  (CallFunction|SetHealth (- (Variables|Default|GetCurrentHealth) InAmount)))