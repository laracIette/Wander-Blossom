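; BP_GuardMagnet is a trap actor that captures one designated guard and pulls it onto itself.
; When the TargetGuard's capsule enters the Box, it latches HasGuard, deactivates the guard's movement and disables the guard.
; A timeline then lerps the guard from its captured location and rotation to the magnet's own transform, taking the shortest rotation path.
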(event OnComponentBeginOverlap(Box)
  (params (OverlappedComponent :type Primitive%20Component%20Object%20Reference) (OtherActor :type Actor%20Object%20Reference) (OtherComp :type Primitive%20Component%20Object%20Reference) (OtherBodyIndex :type Integer) (bFromSweep :type Boolean) (SweepResult :type Hit%20Result%20Structure%20%28by%20ref%29))
  (if (not (Variables|Default|GetbHasGuard))
    (bind _targetguard (Variables|Default|GetTargetGuard)
      (:then
        (if (== (Variables|/Script/Engine.Character|GetCapsuleComponent _targetguard) OtherComp)
          (Variables|Default|SetbHasGuard true)
          (Components|Activation|Deactivate (Variables|/Script/Engine.Character|GetCharacterMovement _targetguard))
          (Default|Disable _targetguard)
          (bind _returnvalue (Transformation|GetActorRotation _targetguard))
          (bind _returnvalue_2 (Transformation|GetActorLocation _targetguard))
          (bind _alpha (Timeline|AttractGuardTimeline Play)
            (:Update
              (Transformation|SetActorLocationAndRotation _targetguard (Math|Vector|Lerp(Vector) _returnvalue_2 (Transformation|GetActorLocation) _alpha) (Math|Rotator|Lerp(Rotator) _returnvalue (Transformation|GetActorRotation) _alpha true))))))
      (:else))))

(fn ConstructionScript)