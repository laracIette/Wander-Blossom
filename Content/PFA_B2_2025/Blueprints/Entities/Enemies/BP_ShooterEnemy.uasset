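; Ranged enemy that charges a laser at the player and can run away.
; While aggroed with line of sight, it faces the player and plays a cooldown-scaled timeline driving the Niagara beam's alpha, stopping and resetting when either condition is lost.
; Timeline completion submits an AttackComponent attack, which plays feedback and damages the player if still visible.
; BeginRunaway repeatedly AI-moves it to points directly away from the player while the flag holds.
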(event OnAttack(AttackComponent)
  (Default|Play (Variables|Default|GetAttackVisualFeedback) false)
  (Default|Play3D (Variables|Default|GetAttackSoundComponent))
  (bind _boutresult (CallFunction|GetCanSeePlayer))
  (if _boutresult
    (Default|CallOnDealDamage (Variables|Default|GetAttackComponent))))

(event OnDealDamage(AttackComponent)
  (bind _outdamagereceived (Default|ReceiveDamage (Variables|/Game/PFA_B2_2025/Blueprints/Entities/Player/BP_Player.BP_Player_C|GetHealthComponent (Utilities|GetPlayer)) 1))
  (if (> _outdamagereceived 0)
    _))

(event Custom|BeginRunaway
  (Variables|Runaway|SetbIsRunningAway true)
  (AI|AIMoveTo (AI|GetAIController self) (CallFunction|GetRunawayLocation) 0 -1.0 "Default" "Default" true true :!label _label ; Executes only if it finds a point
    (:OnRequestFailed
      (Utilities|FlowControl|DelayUntilNextTick))
    (:OnMoveFinished
      _))
  (if (Variables|Runaway|GetbIsRunningAway)
    (goto _label)))

(event EventTick
  (params (DeltaSeconds :type Float%20%28single-precision%29))
  (if (CallFunction|GetIsAggro)
    (bind (_boutresult _outhitlocation) (CallFunction|GetCanSeePlayer))
    (if _boutresult
      (CallFunction|LookatPlayer 1.0)
      (Class|NiagaraComponent|SetVariablePosition (Variables|Default|GetLaserNiagaraSystem) "Beam End" _outhitlocation)
      (bind _value (Timeline|LaserAlphaTimeline Play)
        (:Update
          (Niagara|SetNiagaraVariable(Float) (Variables|Default|GetLaserNiagaraSystem) "Beam Alpha" _value))
        (:Finished
          (Default|SubmitAttack (Variables|Default|GetAttackComponent))
          (Components|Timeline|SetPlaybackPosition (Variables|Default|GetLaserAlphaTimeline) 0.0 false true)))
      (else
        (Utilities|FlowControl|Sequence :!label _label
          (:then_0
            (Timeline|LaserAlphaTimeline Stop))
          (:then_1
            (Timeline|LaserAlphaTimeline SetNewTime)))))
    (else
      (goto _label))))

(event EventBeginPlay
  (Components|Timeline|SetPlayRate (Variables|Default|GetLaserAlphaTimeline) (/ (Components|Timeline|GetTimelineLength (Variables|Default|GetLaserAlphaTimeline)) (Variables|/Game/PFA_B2_2025/Blueprints/Entities/Attacks/AC_Attack.AC_Attack_C|GetAttackCooldown (Variables|Default|GetAttackComponent)))))

(fn ConstructionScript
  (|CallParentFunction))

(fn GetRunawayLocation
  (return (+ (Transformation|GetActorLocation) (* (CallFunction|GetDirectiontoPlayer) (Math|Float|MakeLiteralFloat (Variables|Runaway|GetRunawayDistance))))))

(fn GetDirectiontoPlayer
  (return (Math|Vector|GetUnitDirection(Vector) (Transformation|GetActorLocation (Utilities|GetPlayer)) (Transformation|GetActorLocation))))

(fn GetCanSeePlayer
  (bind _outhit (Collision|LineTraceByChannel (Transformation|GetActorLocation) (Transformation|GetActorLocation (Utilities|GetPlayer)) "TraceTypeQuery2" true 0 "None" true "(R=1.000000,G=0.000000,B=0.000000,A=1.000000)" "(R=0.000000,G=1.000000,B=0.000000,A=1.000000)" 0.5))
  (if (== (.HitActor (Collision|BreakHitResult _outhit)) (Utilities|GetPlayer))
    (return true (Transformation|GetActorLocation (Utilities|GetPlayer)))
    (else
      (return false (.Location (Collision|BreakHitResult _outhit))))))