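; BP_Enemy is an enemy actor with health, aggro detection and helpers for facing the player.
; Damage is printed; death destroys it after a short delay and, if the player lacks full health, spawns a health collectible that the player immediately collects.
; Helpers yaw toward the player by alpha, test aggro collider overlap and expose a look-at point.
; Overlapping a "kill"-tagged actor while alive plays death visual feedback.
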(event OnComponentBeginOverlap(CapsuleComponent)
  (params (OverlappedComponent :type Primitive%20Component%20Object%20Reference) (OtherActor :type Actor%20Object%20Reference) (OtherComp :type Primitive%20Component%20Object%20Reference) (OtherBodyIndex :type Integer) (bFromSweep :type Boolean) (SweepResult :type Hit%20Result%20Structure%20%28by%20ref%29))
  (if (Default|GetIsAlive (Variables|Default|GetHealthComponent))
    (if (Actor|ActorHasTag OtherActor "kill")
      (Default|Play (Variables|Default|GetDeathVisualFeedback) false))))

(event OnReceiveDamage(HealthComponent)
  (params (InAmount :type Integer))
  (Development|PrintText (Utilities|Text|FormatText "Enemy {Name} received {Damage} damage. Remaining health: {Health}" (Utilities|GetDisplayName self) InAmount (Variables|/Game/PFA_B2_2025/Blueprints/Entities/Health/AC_Health.AC_Health_C|GetCurrentHealth (Variables|Default|GetHealthComponent)))))

(event OnDie(HealthComponent)
  (bind _outplayer (Utilities|GetPlayer))
  (bind _healthcomponent (Variables|/Game/PFA_B2_2025/Blueprints/Entities/Player/BP_Player.BP_Player_C|GetHealthComponent _outplayer))
  (Utilities|FlowControl|Delay 0.2)
  (Actor|DestroyActor)
  (if (< (Variables|/Game/PFA_B2_2025/Blueprints/Entities/Health/AC_Health.AC_Health_C|GetCurrentHealth _healthcomponent) (Variables|/Game/PFA_B2_2025/Blueprints/Entities/Health/AC_Health.AC_Health_C|GetMaxHealth _healthcomponent))
    (bind _returnvalue (Game|SpawnActorfromClass "/Game/PFA_B2_2025/Blueprints/Interactables/Collectible/BP_HealthCollectible.BP_HealthCollectible_C" (Transformation|GetActorTransform) "AlwaysSpawn" "MultiplyWithRoot" 0 0))
    (Default|CollectCollectible (Utilities|GetPlayer) _returnvalue)))

(fn ConstructionScript)

(fn LookatPlayer
  (params (InAlpha :type Float%20%28double-precision%29))
  (bind _returnvalue (Transformation|GetActorRotation))
  (Transformation|SetActorRotation (Math|Rotator|MakeRotator (.roll _returnvalue) (.pitch _returnvalue) (Math|Float|Lerp (.yaw (Transformation|GetActorRotation)) (.yaw (Math|Rotator|FindLookatRotation (Transformation|GetActorLocation) (Transformation|GetActorLocation (Utilities|GetPlayer)))) InAlpha))))

(fn GetIsAggro
  (return (Class|PrimitiveComponent|IsOverlappingComponent (Variables|Default|GetAggroCollider) (Variables|/Script/Engine.Character|GetCapsuleComponent (Utilities|GetPlayer)))))

(fn GetLookatLocation
  (return (Transformation|GetWorldLocation (Variables|Default|GetLookAtPosition))))