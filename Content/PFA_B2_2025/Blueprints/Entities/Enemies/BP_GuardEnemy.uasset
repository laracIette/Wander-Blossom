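; Guard enemy that stalks the player while aggroed, deals contact damage and knocks the player away.
; Tick starts or stops continuous AI MoveTo pursuit based on aggro and a CanStalk flag.
; Attack collider overlaps submit attacks through AttackComponent, dealing damage with visual feedback and a launch on successful hits.
; A separate launch collider pauses stalking and plays a timeline-driven sine shake, launching the player if they remain until it finishes.
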(event OnAttack(AttackComponent)
  (Default|CallOnDealDamage (Variables|Default|GetAttackComponent)))

(event OnComponentBeginOverlap(AttackCollider)
  (params (OverlappedComponent :type Primitive%20Component%20Object%20Reference) (OtherActor :type Actor%20Object%20Reference) (OtherComp :type Primitive%20Component%20Object%20Reference) (OtherBodyIndex :type Integer) (bFromSweep :type Boolean) (SweepResult :type Hit%20Result%20Structure%20%28by%20ref%29))
  (bind _asbp_player (Utilities|Casting|CastToBP_Player OtherActor))
  (if (== (Variables|/Script/Engine.Character|GetCapsuleComponent _asbp_player) OtherComp)
    (Default|SubmitAttack (Variables|Default|GetAttackComponent))))

(event OnDealDamage(AttackComponent)
  (bind _outdamagereceived (Default|ReceiveDamage (Variables|/Game/PFA_B2_2025/Blueprints/Entities/Player/BP_Player.BP_Player_C|GetHealthComponent (Utilities|GetPlayer)) 1))
  (if (> _outdamagereceived 0)
    (Default|Play (Variables|Default|GetAttackVisualFeedback) false)
    (CallFunction|LaunchPlayer)))

(event OnComponentBeginOverlap(LaunchPlayerCollider)
  (params (OverlappedComponent :type Primitive%20Component%20Object%20Reference) (OtherActor :type Actor%20Object%20Reference) (OtherComp :type Primitive%20Component%20Object%20Reference) (OtherBodyIndex :type Integer) (bFromSweep :type Boolean) (SweepResult :type Hit%20Result%20Structure%20%28by%20ref%29))
  ;[0.15 0.15 0.15 0.5] Launch Player
  (bind _asbp_player (Utilities|Casting|CastToBP_Player OtherActor))
  (if (== (Variables|/Script/Engine.Character|GetCapsuleComponent _asbp_player) OtherComp)
    (Variables|Default|SetbCanStalk false)
    (bind _returnvalue (Transformation|GetActorLocation))
    (bind _returnvalue_2 (Transformation|GetActorRightVector))
    (bind _speed (Timeline|ShakeTimeline PlayFromStart)
      (:Update
        (Transformation|SetActorLocation (+ _returnvalue (* _returnvalue_2 (* (Math|Trig|Sin(Radians) (* (Utilities|Time|GetGameTimeinSeconds) (Math|Float|Power _speed 2.0))) (* (Variables|Default|GetShakeRange) _speed)))) false false))
      (:Finished
        (CallFunction|LaunchPlayer)))))

(event OnComponentEndOverlap(LaunchPlayerCollider)
  (params (OverlappedComponent :type Primitive%20Component%20Object%20Reference) (OtherActor :type Actor%20Object%20Reference) (OtherComp :type Primitive%20Component%20Object%20Reference) (OtherBodyIndex :type Integer))
  ;[0.15 0.15 0.15 0.5] Launch Player
  (bind _asbp_player (Utilities|Casting|CastToBP_Player OtherActor))
  (if (== (Variables|/Script/Engine.Character|GetCapsuleComponent _asbp_player) OtherComp)
    (Variables|Default|SetbCanStalk true)
    (bind _speed (Timeline|ShakeTimeline Stop)
      (:Update
        (Transformation|SetActorLocation (+ (stale OnComponentBeginOverlap(LaunchPlayerCollider) _returnvalue) (* (stale OnComponentBeginOverlap(LaunchPlayerCollider) _returnvalue_2) (* (Math|Trig|Sin(Radians) (* (Utilities|Time|GetGameTimeinSeconds) (Math|Float|Power _speed 2.0))) (* (Variables|Default|GetShakeRange) _speed)))) false false))
      (:Finished
        (CallFunction|LaunchPlayer)))))

(event Custom|LaunchPlayer
  ;[0.15 0.15 0.15 0.5] Launch Player
  (Character|LaunchCharacter (Utilities|GetPlayer) (* (Math|Vector|GetUnitDirection(Vector) (Transformation|GetActorLocation) (Transformation|GetActorLocation (Utilities|GetPlayer))) (Variables|Default|GetLaunchPlayerForce)) true true))

(event Custom|Disable
  (CallFunction|EndStalk)
  (CallFunction|ResetVelocity))

(event Custom|EndStalk
  (if (Variables|Default|GetbIsStalking)
    (Variables|Default|SetbIsStalking false)
    (AI|Navigation|StopMovement (AI|GetAIController self))))

(event Custom|BeginStalk
  (if (not (Variables|Default|GetbIsStalking))
    (Variables|Default|SetbIsStalking true)
    (Default|ResetLastAttackTime (Variables|Default|GetAttackComponent)) ; todo: why?
    (AI|AIMoveTo (AI|GetAIController self) "0, 0, 0" (Utilities|GetPlayer) -1.0 "Default" "Default" true true true
      (:OnRequestFailed
        (Variables|Default|SetbIsStalking false)))))

(event Custom|ResetVelocity
  (Variables|/Script/Engine.MovementComponent|SetVelocity (Variables|Character|GetCharacterMovement) "0, 0, 0"))

(event EventTick
  (params (DeltaSeconds :type Float%20%28single-precision%29))
  (if (Variables|Default|GetbCanStalk)
    (if (CallFunction|GetIsAggro) ; todo: maybe check is magnet first
      (CallFunction|BeginStalk)
      (else
        (CallFunction|EndStalk :!label _label)))
    (else
      (goto _label))))

(fn ConstructionScript
  (|CallParentFunction))