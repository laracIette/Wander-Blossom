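; BP_StalkerEnemy is an enemy that follows the player and damages them on attack.
; On BeginPlay it binds handlers to player overlap and alignment events from its parent.
; Stalking starts and stops an AI MoveTo toward the player.
; Attacks go through an AttackComponent, whose OnAttack applies damage to the player's HealthComponent and plays visual feedback when damage lands.
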(event OnAttack(AttackComponent)
  (bind _outdamagereceived (Default|ReceiveDamage (Variables|/Game/PFA_B2_2025/Blueprints/Entities/Player/BP_Player.BP_Player_C|GetHealthComponent (Utilities|GetPlayer)) 1.0))
  (if (> _outdamagereceived 0.0)
    (Default|Play (Variables|Default|GetAttackVisualFeedback))))

(event Custom|EndStalk
  (AI|Navigation|StopMovement (AI|GetAIController self)))

(event Custom|BeginStalk
  (AI|AIMoveTo (AI|GetAIController self) "0, 0, 0" (Utilities|GetPlayer) -1.0 "Default" "Default" true true true))

(event Custom|Attack
  (Default|EventSubmitAttack (Variables|Default|GetAttackComponent)))

(event EventBeginPlay
  (EventDispatchers|BindEventtoOnBeginOverlapPlayer (EventDispatchers|CreateEvent :!event Custom|BeginStalk))
  (EventDispatchers|BindEventtoOnEndOverlapPlayer (EventDispatchers|CreateEvent :!event Custom|EndStalk))
  (EventDispatchers|BindEventtoOnAlignedwithPlayer (EventDispatchers|CreateEvent :!event Custom|Attack)))

(fn ConstructionScript
  (|CallParentFunction))