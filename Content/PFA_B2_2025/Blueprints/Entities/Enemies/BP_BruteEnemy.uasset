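; Brute enemy that stalks the player and, when aggroed, performs a leaping plunge attack.
; Montage notifies drive timelines: a trace-limited jump, a tracking phase with a decal on the player's feet, then a plunge to a traced point or one-time forced target.
; Landing damages and knocks back an overlapping player and destroys overlapping destructibles, then stalking resumes.
; Death stops the timelines and plays a KO montage.
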(event OnAttack(AttackComponent)
  ;[0.15 0.15 0.15 0.5] 2. Attack
  (if (Default|GetIsAlive (Variables|Default|GetHealthComponent))
    (CallFunction|EndStalk)
    (CallFunction|OrienttoMovement false)
    (Variables|/Script/Engine.CharacterMovementComponent|SetGravityScale (Variables|Character|GetCharacterMovement) 0.0)
    (Animation|PlayAnimMontage "/Game/PFA_B2_2025/Animations/Brute/AM_BruteAttack.AM_BruteAttack" 1.0 "None")))

(event OnDie(HealthComponent)
  (Audio|Components|Audio|Stop (Variables|Default|GetLookAtPlayerTimeline))
  (CallFunction|EndStalk)
  (CallFunction|DestroyTargetDecal)
  (Animation|PlayAnimMontage "/Game/PFA_B2_2025/Animations/Brute/AM_BruteKO.AM_BruteKO" 1.0 "None")
  (CallFunction|PlaySound "/Game/PFA_B2_2025/Audio/SFX/Enemies/Creature/MS_CreatureDie.MS_CreatureDie"))

(event OnDealDamage(AttackComponent)
  (bind _returnvalue (Transformation|GetActorLocation))
  (bind _outplayer (Utilities|GetPlayer))
  (bind _outplayer_2 (Utilities|GetPlayer))
  (bind _returnvalue_2 (Transformation|GetActorLocation _outplayer_2))
  (bind _returnvalue_3 (Math|Vector|GetUnitDirection(Vector) _returnvalue _returnvalue_2))
  ;[0.15 0.15 0.15 0.5] 6. Damage
  (Utilities|FlowControl|Sequence
    (:then_0
      ;;[0.15 0.15 0.15 0.5] Damage Player
      (if (Class|PrimitiveComponent|IsOverlappingComponent (Variables|Default|GetAttackCollider) (Variables|/Script/Engine.Character|GetCapsuleComponent _outplayer))
        (bind _outdamagereceived (Default|ReceiveDamage (Variables|/Game/PFA_B2_2025/Blueprints/Entities/Player/BP_Player.BP_Player_C|GetHealthComponent _outplayer) 1))
        (if (> _outdamagereceived 0)
          (Niagara|SpawnSystematLocation (Variables|Default|GetAttackNiagaraSystem) (Transformation|GetActorLocation))
          (Character|LaunchCharacter (Utilities|GetPlayer) (* (Math|Vector|Normalize (Math|Vector|MakeVector (.x _returnvalue_3) (.y _returnvalue_3) 0.0)) (Variables|Default|GetLaunchPlayerForce)) true false))))
    (:then_1
      ;;[0.15 0.15 0.15 0.5] Destroy Destructibles
      (for _array_element (Collision|GetOverlappingActors (Variables|Default|GetAttackCollider) "/Game/PFA_B2_2025/Blueprints/Interactables/Destructibles/BP_Destructible.BP_Destructible_C" :!class /Script/Engine.PrimitiveComponent)
        (Default|Destroy (.AsBP%20Destructible (Utilities|Casting|CastToBP_Destructible _array_element)))))
    (:then_2
      (CallFunction|ResetMovement))))

(event OnReceiveDamage(HealthComponent)
  (params (InAmount :type Integer))
  (if (Default|GetIsAlive (Variables|Default|GetHealthComponent))
    (CallFunction|PlaySound "/Game/PFA_B2_2025/Audio/SFX/Enemies/Creature/MS_CreatureHit.MS_CreatureHit")))

(event Custom|OrientToMovement
  (params (bInValue :type Boolean))
  (Variables|/Script/Engine.CharacterMovementComponent|SetbOrientRotationToMovement (Variables|Character|GetCharacterMovement) bInValue)
  (Variables|Default|SetbUseControllerRotationYaw (not bInValue)))

(event Custom|SpawnTargetDecal
  (bind _returnvalue (Class|GameplayStatics|SpawnDecalAttached "/Game/PFA_B2_2025/Materials/Decals/BruteTarget/MI_BruteTarget.MI_BruteTarget" "120.000000,120.000000,20.000000" (Variables|/Game/PFA_B2_2025/Blueprints/Entities/Player/BP_Player.BP_Player_C|GetFeetPosition (Utilities|GetPlayer)) "None" "0, 0, 0" "0, 0, 0" "KeepRelativeOffset" 0.0))
  (Variables|Default|SetTargetDecal _returnvalue)
  (bind _scale (Timeline|TargetDecalTimeline PlayFromStart)
    (:Update
      (Rendering|Material|SetScalarParameterValue "/Game/PFA_B2_2025/Materials/Decals/BruteTarget/MPC_BruteTarget.MPC_BruteTarget" "Scale" _scale :!class /Script/Engine.KismetMaterialLibrary))))

(event Custom|NotifyBeginLookAtPlayer
  ;[0.15 0.15 0.15 0.5] 4. Look At Player
  (CallFunction|SpawnTargetDecal)
  (Timeline|LookAtPlayerTimeline PlayFromStart
    (:Update
      (CallFunction|LookatPlayer 0.5))
    (:Finished
      (CallFunction|DetachTargetDecal)
      (bind _outlocation (CallFunction|GetPlungeLocation))
      (Utilities|FlowControl|Delay 0.4)
      (if (Default|GetIsAlive (Variables|Default|GetHealthComponent))
        (Animation|PlayAnimMontage "/Game/PFA_B2_2025/Animations/Brute/AM_BruteAttack.AM_BruteAttack" 1.0 "Plunge")))))

(event Custom|EndStalk
  (if (Variables|Default|GetbIsStalking)
    (Variables|Default|SetbIsStalking false)
    (AI|Navigation|StopMovement (AI|GetAIController self))))

(event Custom|BeginStalk
  (if (Default|GetIsAlive (Variables|Default|GetHealthComponent))
    (if (not (Variables|Default|GetbIsStalking))
      (Variables|Default|SetbIsStalking true)
      (AI|AIMoveTo (AI|GetAIController self) "0, 0, 0" (Utilities|GetPlayer) -1.0 "Default" "Default" true true true))))

(event Custom|DetachTargetDecal
  (bind _targetdecal (Variables|Default|GetTargetDecal)
    (:then
      (Transformation|DetachFromComponent _targetdecal "KeepWorld" "KeepWorld" "KeepWorld" true))
    (:else)))

(event Custom|DestroyTargetDecal
  (bind _targetdecal (Variables|Default|GetTargetDecal)
    (:then
      (Components|DestroyComponent _targetdecal)
      (Variables|Default|SetTargetDecal 0))
    (:else)))

(event Custom|ResetMovement
  (Variables|/Script/Engine.CharacterMovementComponent|SetGravityScale (Variables|Character|GetCharacterMovement) 1.0)
  (CallFunction|DestroyTargetDecal)
  (Utilities|FlowControl|Delay 1.0)
  (CallFunction|BeginStalk)
  (CallFunction|OrienttoMovement true))

(event Custom|NotifyJump
  (bind _returnvalue (Transformation|GetActorForwardVector))
  ;[0.15 0.15 0.15 0.5] 3. Jump
  (Variables|/Script/Engine.MovementComponent|SetVelocity (Variables|Character|GetCharacterMovement) "0, 0, 0")
  (bind _returnvalue_2 (Transformation|GetActorLocation))
  (bind _location (CallFunction|GetFurthestReachableLocation (+ (Transformation|GetActorLocation) (* (Math|Vector|Normalize (Math|Vector|MakeVector (.x _returnvalue) (.y _returnvalue) 1.0)) (Variables|Default|GetJumpLength)))))
  (bind _alpha (Timeline|JumpTimeline PlayFromStart)
    (:Update
      (Transformation|SetActorLocation (Math|Vector|Lerp(Vector) _returnvalue_2 _location _alpha) false false))))

(event Custom|NotifyPlunge
  ;[0.15 0.15 0.15 0.5] 5. Plunge
  (bind _returnvalue (Transformation|GetActorLocation))
  (bind _alpha (Timeline|PlungeTimeline PlayFromStart)
    (:Update
      (Transformation|SetActorLocation (Math|Vector|Lerp(Vector) _returnvalue (stale Custom|NotifyBeginLookAtPlayer _outlocation) _alpha) false false))
    (:Finished
      (Animation|PlayAnimMontage "/Game/PFA_B2_2025/Animations/Brute/AM_BruteAttack.AM_BruteAttack" 1.0 "Land")
      (Default|CallOnDealDamage (Variables|Default|GetAttackComponent)))))

(event Custom|NotifyDestroy
  (Niagara|SpawnSystematLocation "/Game/PFA_B2_2025/VFX/Explosion/NS_SmokeBurst.NS_SmokeBurst" (Transformation|GetActorLocation))
  (Actor|DestroyActor))

(event EventTick
  (params (DeltaSeconds :type Float%20%28single-precision%29))
  ;[0.15 0.15 0.15 0.5] 1. Submit Attack
  (if (CallFunction|GetIsAggro "NewEnumerator0")
    (Default|SubmitAttack (Variables|Default|GetAttackComponent))))

(fn ConstructionScript
  (|CallParentFunction))

(fn GetFurthestReachableLocation
  (params (InDestination :type Vector))
  (bind (_outhit _returnvalue) (Collision|LineTraceByChannel (Transformation|GetActorLocation) InDestination "TraceTypeQuery1" true 0 "None"))
  (if _returnvalue
    (return (.Location (Collision|BreakHitResult _outhit)))
    (else
      (return InDestination))))

(fn GetLookatLocation
  (return (Transformation|GetWorldLocation (Variables|Default|GetLookAtPosition))))

(fn GetPlungeLocation
  (bind _returnvalue (Transformation|GetActorLocation))
  (Variables|Default|GetForcedFirstTarget
    (:then
      (bind _returnvalue_2 (Transformation|GetActorLocation (Variables|Default|GetForcedFirstTarget)))
      (Variables|Default|SetForcedFirstTarget 0)
      (return _returnvalue_2))
    (:else
      (bind (_outhit _returnvalue_3) (Collision|LineTraceByChannel (Transformation|GetActorLocation) (+ _returnvalue (* (Math|Vector|GetUnitDirection(Vector) _returnvalue (Transformation|GetWorldLocation (Variables|/Game/PFA_B2_2025/Blueprints/Entities/Player/BP_Player.BP_Player_C|GetFeetPosition (Utilities|GetPlayer)))) (Variables|Default|GetLineTraceLength))) "TraceTypeQuery1" true 0 "None"))
      (if _returnvalue_3
        (return (+ (.Location (Collision|BreakHitResult _outhit)) (Math|Vector|MakeVector 0.0 0.0 (Variables|/Script/Engine.CapsuleComponent|GetCapsuleHalfHeight (Variables|Default|GetCapsuleComponent)))))
        (else
          (return (Transformation|GetActorLocation (Utilities|GetPlayer))))))))