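; BP_MerchantStore is a merchant shop trigger that shows the store view and UI while the player stands inside its box.
; On BeginPlay it creates WBP_Merchant and adds it to the viewport fully transparent.
; When the player's capsule enters, the view blends to the store camera, look input is disabled and a timeline fades the widget in.
; Leaving reverses the fade and blends back, re-enabling look after the blend.
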(event OnComponentBeginOverlap(Box)
  (params (OverlappedComponent :type Primitive%20Component%20Object%20Reference) (OtherActor :type Actor%20Object%20Reference) (OtherComp :type Primitive%20Component%20Object%20Reference) (OtherBodyIndex :type Integer) (bFromSweep :type Boolean) (SweepResult :type Hit%20Result%20Structure%20%28by%20ref%29))
  (bind _asbp_player (Utilities|Casting|CastToBP_Player OtherActor))
  (if (== (Variables|/Script/Engine.Character|GetCapsuleComponent _asbp_player) OtherComp)
    (CallFunction|SwitchtoCamera)
    (bind _opacity (Timeline|ShowWidgetTimeline Play)
      (:Update
        (Widget|SetRenderOpacity (Variables|Default|GetMerchantWidget) _opacity)))))

(event OnComponentEndOverlap(Box)
  (params (OverlappedComponent :type Primitive%20Component%20Object%20Reference) (OtherActor :type Actor%20Object%20Reference) (OtherComp :type Primitive%20Component%20Object%20Reference) (OtherBodyIndex :type Integer))
  (bind _asbp_player (Utilities|Casting|CastToBP_Player OtherActor))
  (if (== (Variables|/Script/Engine.Character|GetCapsuleComponent _asbp_player) OtherComp)
    (CallFunction|SwitchtoPlayerCamera)
    (bind _opacity (Timeline|ShowWidgetTimeline Reverse)
      (:Update
        (Widget|SetRenderOpacity (Variables|Default|GetMerchantWidget) _opacity)))))

(event Custom|SwitchToCamera
  (bind _camera (Variables|Default|GetCamera)
    (:then
      (Game|Player|SetViewTargetwithBlend (Game|GetPlayerController 0) _camera (Variables|Default|GetCameraBlendTime) "VTBlend_EaseInOut" 2.0 false)
      (Variables|/Game/PFA_B2_2025/Blueprints/Entities/Player/BP_Player.BP_Player_C|SetbCanLook (Utilities|GetPlayer) false))
    (:else)))

(event Custom|SwitchToPlayerCamera
  (Variables|Default|GetCamera
    (:then
      (Game|Player|SetViewTargetwithBlend (Game|GetPlayerController 0) (Utilities|GetPlayer) (Variables|Default|GetCameraBlendTime) "VTBlend_EaseInOut" 2.0 false)
      (Utilities|FlowControl|Delay (Variables|Default|GetCameraBlendTime))
      (Variables|/Game/PFA_B2_2025/Blueprints/Entities/Player/BP_Player.BP_Player_C|SetbCanLook (Utilities|GetPlayer) true))
    (:else)))

(event EventBeginPlay
  (bind _returnvalue (UserInterface|CreateWidget "/Game/PFA_B2_2025/Widgets/Collectible/WBP_Merchant.WBP_Merchant_C"))
  (bind _output_get (Variables|Default|SetMerchantWidget _returnvalue))
  (UserInterface|Viewport|AddtoViewport _output_get 0)
  (Widget|SetRenderOpacity (Variables|Default|GetMerchantWidget) 0.0))

(fn ConstructionScript)