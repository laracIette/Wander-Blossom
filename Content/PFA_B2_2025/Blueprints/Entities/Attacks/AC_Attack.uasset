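; AC_Attack is an attack component that handles cooldown timing and combo counting, with an empty ResetCombo event as a hook.
; SubmitAttack checks CanAttack, waits out any remaining cooldown, then runs Attack and fires the OnAttack dispatcher.
; Attack records the time, increments the combo and restarts a retriggerable delay.
; When that delay expires, the combo returns to zero, calling ResetCombo and the OnResetCombo dispatcher.
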(event Custom|SubmitAttack
  (if (Utilities|CanAttack)
    (if (Utilities|IsonAttackCooldown)
      (Utilities|FlowControl|Delay (- (Variables|Attack|GetAttackCooldown) (Utilities|TimeSinceLastAttack))))
    (CallFunction|Attack)
    (Default|CallOnAttack)))

(event Custom|Attack
  (Variables|Attack|SetLastAttackTime (Utilities|Time|GetGameTimeinSeconds))
  (Math|Integer|IncrementInt (Variables|Combo|GetCurrentCombo)
    (:%20%20
      (Utilities|FlowControl|RetriggerableDelay (Variables|Combo|GetComboCooldown))
      (Variables|Combo|SetCurrentCombo 0)
      (CallFunction|ResetCombo)
      (Default|CallOnResetCombo))))

(event Custom|ResetCombo)