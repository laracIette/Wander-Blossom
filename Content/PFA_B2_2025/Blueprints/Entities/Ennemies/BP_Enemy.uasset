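; BP_Enemy is an enemy actor that can take damage and die through its HealthComponent.
; On BeginPlay it initializes that component as damageable with a normalized health range and binds its die and receive-damage events.
; Each hit spawns a Niagara burst explosion at the actor's location, scaled by the damage amount.
; Death waits one tick before destroying the actor.
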(event Custom|OnEventDie
  (Utilities|FlowControl|DelayUntilNextTick)
  (Actor|DestroyActor))

(event Custom|OnEventReceiveDamage
  (params (InAmount :type Float%20%28double-precision%29))
  (Niagara|SpawnSystematLocation "/Game/PFA_B2_2025/VFX/Explosion/NS_BurstExplosion.NS_BurstExplosion" (Transformation|GetActorLocation) "0, 0, 0" (Math|Conversions|ToVector(Float) InAmount)))

(event EventBeginPlay
  (Default|Init (Variables|Default|GetHealthComponent) true 0.0 1.0)
  (EventDispatchers|BindEventtoEventDie (Variables|Default|GetHealthComponent) (EventDispatchers|CreateEvent :!event Custom|OnEventDie))
  (EventDispatchers|BindEventtoEventReceiveDamage (Variables|Default|GetHealthComponent) (EventDispatchers|CreateEvent :!event Custom|OnEventReceiveDamage)))

(fn ConstructionScript)