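; Blueprint function library that switches the first local player's input mode between gameplay and UI.
; It offers game-only, UI-only and combined game-and-UI helpers, each setting the input mode on player controller 0 and toggling the mouse cursor to match.
; The two UI variants take a widget to focus and show the cursor, while game-only hides it without flushing input.
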(fn SetInputGameOnly
  (bind ___worldcontext (LocalVariables|Get__WorldContext))
  (bind _returnvalue (Game|GetPlayerController ___worldcontext))
  (Input|SetInputModeGameOnly _returnvalue false)
  (Variables|/Script/Engine.PlayerController|SetbShowMouseCursor _returnvalue false))

(fn SetInputUIOnly
  (params (InWidgetToFocus :type Widget%20Object%20Reference))
  (bind ___worldcontext (LocalVariables|Get__WorldContext))
  (bind _returnvalue (Game|GetPlayerController ___worldcontext))
  (Input|SetInputModeUIOnly _returnvalue InWidgetToFocus "DoNotLock" false)
  (Variables|/Script/Engine.PlayerController|SetbShowMouseCursor _returnvalue true))

(fn SetInputUIandGame
  (params (InWidgetToFocus :type Widget%20Object%20Reference))
  (bind ___worldcontext (LocalVariables|Get__WorldContext))
  (bind _returnvalue (Game|GetPlayerController ___worldcontext))
  (Input|SetInputModeGameandUI _returnvalue InWidgetToFocus "DoNotLock" true false)
  (Variables|/Script/Engine.PlayerController|SetbShowMouseCursor _returnvalue true))