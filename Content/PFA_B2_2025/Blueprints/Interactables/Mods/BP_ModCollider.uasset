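; BP_ModCollider is an interactable trigger that grants the player a movement mod on overlap.
; Its interaction collider casts the overlapping actor to BP_Player and only responds to that player's capsule component.
; A switch on the Mod enum then enables air jump, enables dash, or activates the umbrella, after printing the mod name.
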(event OnComponentBeginOverlap(InteractionCollider)
  (params (OverlappedComponent :type Primitive%20Component%20Object%20Reference) (OtherActor :type Actor%20Object%20Reference) (OtherComp :type Primitive%20Component%20Object%20Reference) (OtherBodyIndex :type Integer) (bFromSweep :type Boolean) (SweepResult :type Hit%20Result%20Structure%20%28by%20ref%29))
  (bind _asbp_player (Utilities|Casting|CastToBP_Player OtherActor))
  (if (== (Variables|/Script/Engine.Character|GetCapsuleComponent _asbp_player) OtherComp)
    (Development|PrintString (Utilities|String|EnumtoString (Variables|Default|GetMod)))
    (switch Utilities|FlowControl|Switch|SwitchonE_Mod (Variables|Default|GetMod)
      (:NewEnumerator0
        (Variables|/Game/PFA_B2_2025/Blueprints/Entities/Player/BP_Player.BP_Player_C|SetbCanAirJump _asbp_player true))
      (:NewEnumerator1
        (Variables|/Game/PFA_B2_2025/Blueprints/Entities/Player/BP_Player.BP_Player_C|SetbCanDash _asbp_player true))
      (:NewEnumerator2
        (Default|ActivateUmbrella _asbp_player)))))

(fn ConstructionScript)