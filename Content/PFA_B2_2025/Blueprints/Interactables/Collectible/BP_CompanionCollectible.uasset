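; Companion collectible that bobs in place and, once collected, follows the player and can be thrown at an enemy.
; A timeline drives the bobbing mesh height, while Tick lerps the collider toward the player's equipped-collectible position.
; Throw launches it with a physics impulse, and the first enemy overlapped is recorded as grabbed, stopping physics until Recall.
; Player attacks on that enemy deal damage through an event bound on timeline updates.
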(event OnComponentBeginOverlap(MeshCollider)
  (params (OverlappedComponent :type Primitive%20Component%20Object%20Reference) (OtherActor :type Actor%20Object%20Reference) (OtherComp :type Primitive%20Component%20Object%20Reference) (OtherBodyIndex :type Integer) (bFromSweep :type Boolean) (SweepResult :type Hit%20Result%20Structure%20%28by%20ref%29))
  (if (Variables|Default|GetbIsThrown)
    (Variables|Default|GetGrabbedEnemy
      (:then)
      (:else
        (bind _asbp_enemy (Utilities|Casting|CastToBP_Enemy OtherActor))
        (CallFunction|GrabEnemy _asbp_enemy)))))

(event Custom|Event%20OnCollected
  ;[0.15 0.15 0.15 0.5] Play explosion particles
  (Default|Play (Variables|Default|GetCollectVisualFeedback))
  ;[0.15 0.15 0.15 0.5] Play explosion sound
  (Default|Play3D (Variables|Default|GetCollectSoundComponent)))

(event Custom|AttackEnemy
  (params (InEnemy :type BP%20Enemy%20Object%20Reference))
  (if (== InEnemy (Variables|Default|GetGrabbedEnemy))
    (bind _grabbedenemy (Variables|Default|GetGrabbedEnemy)
      (:then
        (Default|ReceiveDamage (Variables|/Game/PFA_B2_2025/Blueprints/Entities/Enemies/BP_Enemy.BP_Enemy_C|GetHealthComponent _grabbedenemy) 1.0))
      (:else))))

(event EventTick
  (params (DeltaSeconds :type Float%20%28single-precision%29))
  (if (Variables|Default|GetbIsCollected)
    (if (not (Variables|Default|GetbIsThrown))
      ;[0.15 0.15 0.15 0.5] Set Location
      (Transformation|SetWorldLocation (Variables|Default|GetMeshCollider) (Math|Vector|Lerp(Vector) (Transformation|GetWorldLocation (Variables|Default|GetMeshCollider)) (Transformation|GetWorldLocation (Variables|/Game/PFA_B2_2025/Blueprints/Entities/Player/BP_Player.BP_Player_C|GetEquippedCollectiblePosition (.AsBP%20Player (Utilities|Casting|CastToBP_Player (Game|Player|GetPlayerPawn 0))))) (* (Utilities|Time|GetWorldDeltaSeconds) (Variables|Default|GetFollowSpeed))) false false))))

(event EventBeginPlay
  (bind _mesh (Variables|Default|GetMesh))
  (bind _relativelocation (Variables|/Script/Engine.SceneComponent|GetRelativeLocation _mesh))
  (EventDispatchers|BindEventtoOnCollected (EventDispatchers|CreateEvent :!event Custom|Event%20OnCollected))
  (Variables|Default|SetSphereStartHeight (.z (Variables|/Script/Engine.SceneComponent|GetRelativeLocation (Variables|Default|GetMesh))))
  (Components|Timeline|SetPlayRate (Variables|Default|GetAnimationTimeline) (Variables|Default|GetAnimationTimelinePlayRate))
  (bind _height (Timeline|AnimationTimeline Play)
    (:Update
      (Transformation|SetRelativeLocation _mesh (Math|Vector|MakeVector (.x _relativelocation) (.y _relativelocation) (+ (* _height (Variables|Default|GetSphereHeightRange)) (Variables|Default|GetSphereStartHeight))) false false)
      (EventDispatchers|BindEventtoOnAttackEnemy (.AsBP%20Player (Utilities|Casting|CastToBP_Player (Game|Player|GetPlayerPawn 0))) (EventDispatchers|CreateEvent :!event Custom|AttackEnemy)))))

(fn ConstructionScript)

(fn Throw
  (params (InDirection :type Vector))
  (bind _returnvalue (Math|Vector|Normalize InDirection))
  (Variables|Default|SetbIsThrown true)
  (Audio|Components|Audio|Stop (Variables|Default|GetAnimationTimeline))
  (Physics|SetSimulatePhysics (Variables|Default|GetMeshCollider) true)
  (Physics|AddImpulse (Variables|Default|GetMeshCollider) (* (Variables|Default|GetThrowForce) (Math|Vector|Normalize (Math|Vector|MakeVector (.x _returnvalue) (.y _returnvalue) 0.3))) "None" false))

(fn Recall
  (Variables|Default|SetbIsThrown false)
  (Audio|Components|Audio|Play (Variables|Default|GetAnimationTimeline))
  (Physics|SetSimulatePhysics (Variables|Default|GetMeshCollider) false)
  (Variables|Default|SetGrabbedEnemy 0))

(fn GrabEnemy
  (params (InEnemy :type BP%20Enemy%20Object%20Reference))
  (Variables|Default|SetGrabbedEnemy InEnemy)
  (Physics|SetSimulatePhysics (Variables|Default|GetMeshCollider) false))