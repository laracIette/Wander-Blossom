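; Collectible spawner actor that places a pickup in the level and hands it to the player on approach.
; On BeginPlay it spawns an actor of CollectibleClass at its own location and rotation and keeps a reference.
; When the player's capsule overlaps AttractCollider, it passes that collectible to the player's CollectCollectible and clears the reference, so each spawn is handed over only once.
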(event OnComponentBeginOverlap(AttractCollider)
  (params (OverlappedComponent :type Primitive%20Component%20Object%20Reference) (OtherActor :type Actor%20Object%20Reference) (OtherComp :type Primitive%20Component%20Object%20Reference) (OtherBodyIndex :type Integer) (bFromSweep :type Boolean) (SweepResult :type Hit%20Result%20Structure%20%28by%20ref%29))
  (Variables|Default|GetSpawnedCollectible
    (:then
      (if (== OtherComp (Variables|/Script/Engine.Character|GetCapsuleComponent (Utilities|GetPlayer)))
        (Default|CollectCollectible (Utilities|GetPlayer) (Variables|Default|GetSpawnedCollectible))
        (Variables|Default|SetSpawnedCollectible 0)))
    (:else)))

(event Custom|SpawnCollectible
  (bind _returnvalue (Game|SpawnActorfromClass (Variables|Default|GetCollectibleClass) (Math|Transform|MakeTransform (Transformation|GetActorLocation) (Transformation|GetActorRotation) "1.000000,1.000000,1.000000") "Undefined" "MultiplyWithRoot" 0 0))
  (Variables|Default|SetSpawnedCollectible _returnvalue))

(event EventBeginPlay
  (CallFunction|SpawnCollectible))

(fn ConstructionScript)