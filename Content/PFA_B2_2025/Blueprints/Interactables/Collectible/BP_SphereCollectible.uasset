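; Sphere collectible that bobs in place and plays a destruction effect when collected.
; On BeginPlay it binds to OnCollected and runs a timeline that offsets the mesh height from its starting Z by a configurable range.
; On collection it stops the bob, plays visual and audio feedback, then a second timeline scales the mesh from its current scale before destroying the actor.
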(event Custom|Event%20OnCollected
  (Audio|Components|Audio|Stop (Variables|Default|GetAnimationTimeline))
  ;[0.15 0.15 0.15 0.5] Play explosion particles
  (Default|Play (Variables|Default|GetCollectVisualFeedback))
  ;[0.15 0.15 0.15 0.5] Play explosion sound
  (Audio|Components|Audio|Play (Variables|Default|GetCollectAudio) 0.0)
  (Variables|Default|SetTempSphereStartScale (Variables|/Script/Engine.SceneComponent|GetRelativeScale3D (Variables|Default|GetMesh)))
  (Components|Timeline|SetPlayRate (Variables|Default|GetDestroyTimeline) (Variables|Default|GetDestroyTimelinePlayRate))
  (bind _value (Timeline|DestroyTimeline Play)
    (:Update
      (Transformation|SetRelativeScale3D (Variables|Default|GetMesh) (* _value (Variables|Default|GetTempSphereStartScale))))
    (:Finished
      (Actor|DestroyActor))))

(event EventBeginPlay
  (bind _mesh (Variables|Default|GetMesh))
  (bind _relativelocation (Variables|/Script/Engine.SceneComponent|GetRelativeLocation _mesh))
  (EventDispatchers|BindEventtoOnCollected (EventDispatchers|CreateEvent :!event Custom|Event%20OnCollected))
  (Variables|Default|SetSphereStartHeight (.z (Variables|/Script/Engine.SceneComponent|GetRelativeLocation (Variables|Default|GetMesh))))
  (Components|Timeline|SetPlayRate (Variables|Default|GetAnimationTimeline) (Variables|Default|GetAnimationTimelinePlayRate))
  (bind _height (Timeline|AnimationTimeline Play)
    (:Update
      (Transformation|SetRelativeLocation _mesh (Math|Vector|MakeVector (.x _relativelocation) (.y _relativelocation) (+ (* _height (Variables|Default|GetSphereHeightRange)) (Variables|Default|GetSphereStartHeight))) false false))))

(fn ConstructionScript)