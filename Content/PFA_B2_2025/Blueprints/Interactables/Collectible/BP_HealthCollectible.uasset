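; BP_HealthCollectible is a heart pickup that flies to the player when collected, then destroys itself.
; BeginPlay binds a handler to OnCollected; the Collected event disables heart physics and starts a timeline that lerps the collider's position and look-at rotation toward the player's live location.
; Overlapping the player's capsule only plays the collect sound; no health change happens in this graph.
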(event OnComponentBeginOverlap(HeartCollider)
  (params (OverlappedComponent :type Primitive%20Component%20Object%20Reference) (OtherActor :type Actor%20Object%20Reference) (OtherComp :type Primitive%20Component%20Object%20Reference) (OtherBodyIndex :type Integer) (bFromSweep :type Boolean) (SweepResult :type Hit%20Result%20Structure%20%28by%20ref%29))
  (bind _asbp_player (Utilities|Casting|CastToBP_Player OtherActor))
  (if (== (Variables|/Script/Engine.Character|GetCapsuleComponent _asbp_player) OtherComp)
    (Default|Play3D (Variables|Default|GetCollectSoundComponent))))

(event Custom|Event%20Collected
  (bind _returnvalue (Game|Player|GetPlayerPawn 0))
  (bind _heartcollider (Variables|Default|GetHeartCollider))
  (bind _returnvalue_2 (Transformation|GetWorldLocation _heartcollider))
  (bind _asbp_player (Utilities|Casting|CastToBP_Player _returnvalue))
  (bind _returnvalue_3 (Transformation|GetActorLocation _asbp_player))
  (Physics|SetSimulatePhysics (Variables|Default|GetHeartCollider) false)
  (bind _alpha (Timeline|CollectTimeline Play)
    (:Update
      ;[0.15 0.15 0.15 0.5] Set Location
      (Transformation|SetWorldLocation (Variables|Default|GetHeartCollider) (Math|Vector|Lerp(Vector) _returnvalue_2 _returnvalue_3 _alpha) false false)
      ;[0.15 0.15 0.15 0.5] Set Rotation
      (Transformation|SetWorldRotation (Variables|Default|GetHeartCollider) (Math|Rotator|Lerp(Rotator) (Transformation|GetWorldRotation (Variables|Default|GetHeartCollider)) (Math|Rotator|FindLookatRotation _returnvalue_2 _returnvalue_3) _alpha true) false false))
    (:Finished
      (Actor|DestroyActor) ; todo: eh
    )))

(event EventBeginPlay
  (EventDispatchers|BindEventtoOnCollected (EventDispatchers|CreateEvent :!event Custom|Event%20Collected)))

(fn ConstructionScript)