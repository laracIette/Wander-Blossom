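; Interactable button that toggles on interaction, broadcasting activate and deactivate events, with optional single-use and timed auto-deactivation.
; A timeline scaled to the activation duration drives the mesh's "Pressed" morph target and reverses on deactivation.
; Once the activation delay ends, it fires OnActivate, locks player movement and blends to an optional camera for a set time before returning view and control.
; Single-use buttons disable interaction and clear their overlay material.
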(event Custom|Activate
  (Variables|Default|SetbIsActivated true)
  (Utilities|FlowControl|Sequence
    (:then_0
      (if (Variables|Default|GetbIsSingleUse)
        (Variables|Default|SetbIsInteractable false)
        (Rendering|Material|SetOverlayMaterial (Variables|Default|GetMesh) 0 :!class /Script/Engine.MeshComponent)
        (bind _value (Timeline|ActivateTimeline Play)
          (:Update
            (Components|SkeletalMesh|SetMorphTarget (Variables|Default|GetMesh) "Pressed" _value true)))
        (else
          (Timeline|ActivateTimeline Play))))
    (:then_1
      (Utilities|FlowControl|Delay (Variables|Default|GetActivationDuration))
      (Default|CallOnActivate)
      (CallFunction|SwitchtoButtonCamera)
      (Variables|/Game/PFA_B2_2025/Blueprints/Entities/Player/BP_Player.BP_Player_C|SetbCanMove (Utilities|GetPlayer) false)
      (Utilities|FlowControl|Delay (Variables|Default|GetCameraTime))
      (CallFunction|SwitchtoPlayerCamera)
      (Variables|/Game/PFA_B2_2025/Blueprints/Entities/Player/BP_Player.BP_Player_C|SetbCanMove (Utilities|GetPlayer) true))))

(event Custom|Deactivate
  (Variables|Default|SetbIsActivated false)
  (Default|CallOnDeactivate)
  (bind _value (Timeline|ActivateTimeline Reverse)
    (:Update
      (Components|SkeletalMesh|SetMorphTarget (Variables|Default|GetMesh) "Pressed" _value true))))

(event Custom|SwitchToButtonCamera
  (bind _camera (Variables|Default|GetCamera)
    (:then
      (Game|Player|SetViewTargetwithBlend (Game|GetPlayerController 0) _camera (Variables|Default|GetCameraBlendTime) "VTBlend_EaseInOut" 2.0 false))
    (:else)))

(event Custom|SwitchToPlayerCamera
  (Variables|Default|GetCamera
    (:then
      (Game|Player|SetViewTargetwithBlend (Game|GetPlayerController 0) (Utilities|GetPlayer) (Variables|Default|GetCameraBlendTime) "VTBlend_EaseInOut" 2.0 false))
    (:else)))

(event EventBeginPlay
  (|CallParentFunction)
  (EventDispatchers|BindEventtoOnDeactivate (EventDispatchers|CreateEvent :!event Custom|Deactivate))
  (Components|Timeline|SetPlayRate (Variables|Default|GetActivateTimeline) (/ 1.0 (Variables|Default|GetActivationDuration))))

(event EventInteract
  (|CallParentFunction)
  (if (Variables|Default|GetbIsInteractable)
    (if (Variables|Default|GetbIsActivated)
      (CallFunction|Deactivate :!label _label)
      (else
        (CallFunction|Activate)
        (if (Variables|Default|GetbIsAutoDeactivate)
          (Utilities|FlowControl|RetriggerableDelay (Variables|Default|GetActivationDuration))
          (goto _label))))))

(fn ConstructionScript
  (|CallParentFunction))

(fn GetMeshComponent
  (return (Variables|Default|GetMesh)))