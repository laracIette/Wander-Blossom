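; BP_End is the end-of-game trigger that brings up the end screen for the player.
; Overlapping UnlockCollider with the BP_Player capsule sets IsUnlocked, arming the second trigger.
; When the capsule then enters CinematicCollider, the game pauses, creates WBP_End, adds it to the viewport and switches input to UI only.
; Both overlaps compare against the capsule component, so other player components are ignored.
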(event OnComponentBeginOverlap(UnlockCollider)
  (params (OverlappedComponent :type Primitive%20Component%20Object%20Reference) (OtherActor :type Actor%20Object%20Reference) (OtherComp :type Primitive%20Component%20Object%20Reference) (OtherBodyIndex :type Integer) (bFromSweep :type Boolean) (SweepResult :type Hit%20Result%20Structure%20%28by%20ref%29))
  (bind _asbp_player (Utilities|Casting|CastToBP_Player OtherActor))
  (if (== (Variables|/Script/Engine.Character|GetCapsuleComponent _asbp_player) OtherComp)
    (Variables|Default|SetbIsUnlocked true)))

(event OnComponentBeginOverlap(CinematicCollider)
  (params (OverlappedComponent :type Primitive%20Component%20Object%20Reference) (OtherActor :type Actor%20Object%20Reference) (OtherComp :type Primitive%20Component%20Object%20Reference) (OtherBodyIndex :type Integer) (bFromSweep :type Boolean) (SweepResult :type Hit%20Result%20Structure%20%28by%20ref%29))
  (bind _asbp_player (Utilities|Casting|CastToBP_Player OtherActor))
  (if (== (Variables|/Script/Engine.Character|GetCapsuleComponent _asbp_player) OtherComp)
    (if (Variables|Default|GetbIsUnlocked)
      (Game|SetGamePaused true)
      (bind _returnvalue (UserInterface|CreateWidget "/Game/PFA_B2_2025/Widgets/End/WBP_End.WBP_End_C"))
      (UserInterface|Viewport|AddtoViewport _returnvalue 0)
      (CallFunction|SetInputUIOnly _returnvalue))))

(fn ConstructionScript)